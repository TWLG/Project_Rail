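; GM_BASE is a free-moving camera Blueprint driven by two movement input axes.
; Each axis event offsets the Camera component in world space along its own forward or right vector, scaled by axis value and Speed.
; Movement teleports without sweeping and is not scaled by delta time.
; Both axis events then feed a shared debug print of "Hello".
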(event Input|AxisEvents|InputAxisForwardsandBackwards
  (params (AxisValue :type Float%20%28single-precision%29))
  (Transformation|AddWorldOffset (Variables|Default|GetCamera) (* (Math|Vector|GetForwardVector (Transformation|GetWorldRotation (Variables|Default|GetCamera))) (* AxisValue (Variables|Default|GetSpeed))) false true)
  (Development|PrintString "Hello"))

(event Input|AxisEvents|InputAxisLeftandRight
  (params (AxisValue :type Float%20%28single-precision%29))
  (Transformation|AddWorldOffset (Variables|Default|GetCamera) (* (Math|Vector|GetRightVector (Transformation|GetWorldRotation (Variables|Default|GetCamera))) (* AxisValue (Variables|Default|GetSpeed))) false true)
  (Development|PrintString "Hello"))

(fn ConstructionScript)